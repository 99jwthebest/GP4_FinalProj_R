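; Radio component that plays random songs from a song list back to back as non-spatial 2D audio.
; From BeginPlay, ChangeSong spawns a sound, stores it as the current song, waits, then calls itself again.
; The wait takes its duration from a second random SelectNewSong call, so it can differ from the playing song's length.
; A fade-out of the current song exists but is never run.
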(event Custom|ChangeSong
  (bind _selectedsong (CallFunction|SelectNewSong))
  (Development|PrintString "Playing New Song")
  (bind _returnvalue (Audio|SpawnSound2D _selectedsong (Variables|Default|GetVolume%20Multiplier) 1.0 0.0 0))
  (Variables|Default|SetCurrentSongRef _returnvalue)
  (Utilities|FlowControl|Delay (Variables|/Script/Engine.SoundBase|GetDuration _selectedsong))
  (CallFunction|ChangeSong))

(event EventBeginPlay
  (CallFunction|ChangeSong))

(event EventTick
  (params (DeltaSeconds :type Float%20%28single-precision%29)))

(fn SelectNewSong
  (bind _songlist (Variables|Default|GetSongList))
  (Variables|Default|SetProvisionalSong (Utilities|Array|Get(acopy) _songlist (Math|Random|RandomIntegerinRange 0 (Utilities|Array|LastIndex _songlist))))
  (return (Variables|Default|GetProvisionalSong)))